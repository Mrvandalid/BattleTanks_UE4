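; Player tank Blueprint that binds input for orbiting the camera, driving and firing.
; On BeginPlay it hands the barrel and turret to TankAiming and both tracks to TankMovement.
; Frame-time-scaled aim axes accumulate yaw and clamped pitch into the spring arm's relative rotation, while Fire calls TankAiming.
; Driving supports either direct per-track throttle or forward and turn intents sent through TankMovement.
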(event EventBeginPlay
  (Class|TankAimingComponent|Initialize (Variables|Default|GetTankAiming) (Variables|Default|GetBarrel) (Variables|Default|GetTankTurret))
  (Class|TankMovementComponent|Initialize (Variables|Default|GetTankMovement) (Variables|Default|GetTankTrackL) (Variables|Default|GetTankTrackR)))

(event Input|ActionEvents|InputActionFire
  (params (Key :type Key%20Structure :default "AnyKey"))
  ;[1 1 1] Fire
  (:Pressed
    (Class|TankAimingComponent|Fire (Variables|Default|GetTankAiming))))

(event Input|AxisEvents|InputAxisLeftTrackThrottle
  (params (AxisValue :type Float%20%28single-precision%29))
  ;[1 1 1] Setup Movement
  (Class|TankTrack|SetThrottle (Variables|Default|GetTankTrackL) AxisValue))

(event Input|AxisEvents|InputAxisRightTrackThrottle
  (params (AxisValue :type Float%20%28single-precision%29))
  ;[1 1 1] Setup Movement
  (Class|TankTrack|SetThrottle (Variables|Default|GetTankTrackR) AxisValue))

(event Input|AxisEvents|InputAxisMoveForward
  (params (AxisValue :type Float%20%28single-precision%29))
  ;[1 1 1] Setup Movement
  (Class|TankMovementComponent|IntendMoveForward (Variables|Default|GetTankMovement) AxisValue))

(event Input|AxisEvents|InputAxisTurnRight
  (params (AxisValue :type Float%20%28single-precision%29))
  ;[1 1 1] Setup Movement
  (Class|TankMovementComponent|IntendTurnRight (Variables|Default|GetTankMovement) AxisValue))

(event Input|AxisEvents|InputAxisAim_Vertical
  (params (AxisValue :type Float%20%28single-precision%29))
  ;[1 1 1] Camera Input Binding
  (bind _output_get (Variables|Default|SetPitchVariable (Math|Float|Clamp(Float) (+ (stale _output_get) (* AxisValue (Utilities|Time|GetWorldDeltaSeconds) 5e+01)) -6e+01 35.0)))
  (Transformation|SetRelativeRotation (Variables|Default|GetSpringArm) (Math|Rotator|MakeRotator 0.0 _output_get (stale Input|AxisEvents|InputAxisAim_Azimuth _output_get)) false false))

(event Input|AxisEvents|InputAxisAim_Azimuth
  (params (AxisValue :type Float%20%28single-precision%29))
  ;[1 1 1] Camera Input Binding
  (bind _output_get (Variables|Default|SetYawVariable (+ (stale _output_get) (* (Utilities|Time|GetWorldDeltaSeconds) AxisValue 5e+01))))
  (Transformation|SetRelativeRotation (Variables|Default|GetSpringArm) (Math|Rotator|MakeRotator 0.0 (stale Input|AxisEvents|InputAxisAim_Vertical _output_get) _output_get) false false))

(fn ConstructionScript)